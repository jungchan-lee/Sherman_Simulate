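; VR hand crank for the tank turret that turns the gun barrel, apparently for vertical aiming, while grabbed.
; Grabbing shows a left-hand mesh and starts a looping UpdateRotation timer; dropping hides it and pauses the timer.
; Each tick smooths a look-at dot product toward the motion controller into wheel spin, matches the hand's pitch, and maps that spin to a small, clamped barrel roll offset.
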(event OnGrabbed(GrabComponent)
  (params (MotionControllerRight :type Motion%20Controller%20Component%20Object%20Reference) (MotionControllerLeft :type Motion%20Controller%20Component%20Object%20Reference))
  (Variables|Default|SetMotion%20Controller 0)
  (bind _returnvalue (Utilities|Time|SetTimerbyFunctionName 0 "UpdateRotation" 0.02 true))
  (Variables|Default|SetTIme _returnvalue)
  (Rendering|SetVisibility (Variables|Default|GetHandLeft) true false))

(event OnDropped(GrabComponent)
  (Variables|Default|SetMotion%20Controller 0)
  (Class|KismetSystemLibrary|PauseTimer 0 "UpdateRotation")
  (Rendering|SetVisibility (Variables|Default|GetHandLeft) false false))

(event EventBeginPlay
  (Rendering|SetVisibility (Variables|Default|GetHandLeft) false false))

(fn ConstructionScript)

(fn UpdateRotation
  (bind _gunbarrel (Variables|Default|GetGunBarrel))
  (bind _handleft (Variables|Default|GetHandLeft))
  (bind _barrel (Variables|/Game/Tank/BluePrint/BP_GunBarrel.BP_GunBarrel_C|GetBarrel _gunbarrel))
  (bind _relativerotation (Variables|/Script/Engine.SceneComponent|GetRelativeRotation _handleft))
  (bind _returnvalue (Transformation|GetWorldRotation _barrel))
  (bind _output_get (Variables|Default|SetCurrentValue (Math|Interpolation|FInterpTo (Variables|Default|GetCurrentValue) (* (Math|Rotator|NormalizeAxis (Math|Vector|DotProduct (Math|Rotator|GetRotationXVector (Math|Rotator|FindLookatRotation (Transformation|GetWorldLocation (Variables|Default|GetLeftCrankWheel)) (Transformation|GetWorldLocation (Variables|Default|GetMotion%20Controller)))) (Math|Vector|GetForwardVector (Transformation|GetWorldRotation (Variables|Default|GetLeftCrankWheel))))) 5e+02) (Class|KismetSystemLibrary|GetTimerElapsedTimeHandle (Variables|Default|GetTIme)) 4.0)))
  (Variables|Default|SetTurretHandleRotationValue _output_get)
  (Transformation|AddLocalRotation (Variables|Default|GetLeftCrankWheel) (Math|Rotator|MakeRotator 0.0 _output_get 0.0) false false)
  ;[1 1 1] Crank Wheel의 Y축에 따라 Hand Left 메쉬도 같이 움직이게
  (Transformation|SetRelativeRotation _handleft (Math|Rotator|MakeRotator (.roll _relativerotation) (Math|Float|Absolute(Float) (.pitch (Variables|/Script/Engine.SceneComponent|GetRelativeRotation (Variables|Default|GetLeftCrankWheel)))) (.yaw _relativerotation)) false false)
  (Transformation|SetWorldRotation _barrel (Math|Rotator|MakeRotator (+ (Math|Float|MapRangeClamped (.Pitch (Math|Rotator|BreakRotator (Math|Rotator|MakeRotator 0.0 _output_get 0.0))) 3.6e+02 -3.6e+02 1.0 -1.0) (.roll (Variables|/Script/Engine.SceneComponent|GetRelativeRotation (Variables|/Game/Tank/BluePrint/BP_GunBarrel.BP_GunBarrel_C|GetBarrel (Variables|Default|GetGunBarrel))))) (.pitch _returnvalue) (.yaw _returnvalue)) false false))