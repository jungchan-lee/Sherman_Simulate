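; BP_TurnHor_Turret is a grabbable valve that turns the tank turret horizontally, using a motion controller's position.
; Grabbing shows a hand mesh and starts a looping UpdateRotation timer; dropping pauses it and hides the hand.
; Each update eases a turn rate from the valve-to-controller look-at direction, spins the valve and adjusts the hand's roll.
; That rate is clamp-mapped into a small yaw step for the TankTopRotation mesh.
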(event OnGrabbed(GrabComponent)
  (params (MotionControllerRight :type Motion%20Controller%20Component%20Object%20Reference) (MotionControllerLeft :type Motion%20Controller%20Component%20Object%20Reference))
  (Variables|Default|SetMotion%20Controller 0)
  (bind _returnvalue (Utilities|Time|SetTimerbyFunctionName 0 "UpdateRotation" 0.02 true))
  (Variables|Default|SetTIme _returnvalue)
  (Rendering|SetVisibility (Variables|Default|GetHandRight) true false))

(event OnDropped(GrabComponent)
  (Variables|Default|SetMotion%20Controller 0)
  (Class|KismetSystemLibrary|PauseTimer 0 "UpdateRotation")
  (Rendering|SetVisibility (Variables|Default|GetHandRight) false false))

(event EventBeginPlay
  (Rendering|SetVisibility (Variables|Default|GetHandRight) false false))

(event Collision|EventActorBeginOverlap
  (params (OtherActor :type Actor%20Object%20Reference)))

(event EventTick
  (params (DeltaSeconds :type Float%20%28single-precision%29)))

(fn ConstructionScript)

(fn UpdateRotation
  (bind _tanktoprotation (Variables|Default|GetTankTopRotation))
  (bind _handright (Variables|Default|GetHandRight))
  (bind _staticmesh (Variables|/Game/Tank/BluePrint/BP_TankTopRotation.BP_TankTopRotation_C|GetStaticMesh _tanktoprotation))
  (bind _relativerotation (Variables|/Script/Engine.SceneComponent|GetRelativeRotation _handright))
  (bind _returnvalue (Transformation|GetWorldRotation _staticmesh))
  (bind _output_get (Variables|Default|SetCurrentValue (Math|Interpolation|FInterpTo (Variables|Default|GetCurrentValue) (* (Math|Rotator|NormalizeAxis (Math|Vector|DotProduct (Math|Rotator|GetRotationXVector (Math|Rotator|FindLookatRotation (Transformation|GetWorldLocation (Variables|Default|GetValve)) (Transformation|GetWorldLocation (Variables|Default|GetMotion%20Controller)))) (Math|Vector|GetForwardVector (Transformation|GetWorldRotation (Variables|Default|GetValve))))) 5e+02) (Class|KismetSystemLibrary|GetTimerElapsedTimeHandle (Variables|Default|GetTIme)) 4.0)))
  (Transformation|AddLocalRotation (Variables|Default|GetValve) (Math|Rotator|MakeRotator 0.0 _output_get 0.0) false false)
  (Transformation|SetRelativeRotation _handright (Math|Rotator|MakeRotator (Math|Float|Absolute(Float) (* (.pitch (Variables|/Script/Engine.SceneComponent|GetRelativeRotation (Variables|Default|GetValve))) -1.0)) (.pitch _relativerotation) (.yaw _relativerotation)) false false)
  (Transformation|SetWorldRotation _staticmesh (Math|Rotator|MakeRotator (.roll _returnvalue) (.pitch _returnvalue) (+ (Math|Float|MapRangeClamped (.Pitch (Math|Rotator|BreakRotator (Math|Rotator|MakeRotator 0.0 _output_get 0.0))) 3.6e+02 -3.6e+02 1.0 -1.0) (.yaw (Variables|/Script/Engine.SceneComponent|GetRelativeRotation (Variables|/Game/Tank/BluePrint/BP_TankTopRotation.BP_TankTopRotation_C|GetStaticMesh (Variables|Default|GetTankTopRotation)))))) false false))