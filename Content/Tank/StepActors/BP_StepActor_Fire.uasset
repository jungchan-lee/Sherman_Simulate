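; BP_StepActor_Fire is a step actor for the tank's fire step, acting on a breech reference.
; A sphere component's begin overlap calls EventBeginStep, which runs the parent logic, prints a debug message, clears the breech's IsOpen flag and calls its Load function.
; EventEndStep only forwards to the parent, and the end overlap event has no logic.
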(event OnComponentBeginOverlap(Sphere)
  (params (OverlappedComponent :type Primitive%20Component%20Object%20Reference) (OtherActor :type Actor%20Object%20Reference) (OtherComp :type Primitive%20Component%20Object%20Reference) (OtherBodyIndex :type Integer) (bFromSweep :type Boolean) (SweepResult :type Hit%20Result%20Structure%20%28by%20ref%29))
  (CallFunction|EventBeginStep))

(event OnComponentEndOverlap(Sphere)
  (params (OverlappedComponent :type Primitive%20Component%20Object%20Reference) (OtherActor :type Actor%20Object%20Reference) (OtherComp :type Primitive%20Component%20Object%20Reference) (OtherBodyIndex :type Integer)))

(event EventBeginPlay
  (|CallParentFunction) ; This node is disabled and will not be called.\nDrag off pins to build functionality.
)

(event Collision|EventActorBeginOverlap
  (params (OtherActor :type Actor%20Object%20Reference)))

(event EventTick
  (params (DeltaSeconds :type Float%20%28single-precision%29)))

(fn ConstructionScript
  (|CallParentFunction))

(fn EventBeginStep
  (bind _bp_breech (Variables|Default|GetBP_Breech))
  (|CallParentFunction)
  (Development|PrintString "Fire'")
  (Variables|/Game/Tank/BluePrint/BP_Breech.BP_Breech_C|SetIsOpen _bp_breech false)
  (Default|Load _bp_breech))

(fn EventEndStep
  (|CallParentFunction))