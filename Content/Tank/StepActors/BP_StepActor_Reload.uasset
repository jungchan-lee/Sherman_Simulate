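; Tank reload step actor: a motion-controller grab handle that swings to drive loading of the breech.
; While grabbed, it shows a hand mesh and runs EventBeginStep on a fast looping timer; dropping it stops the timer and hides the hand.
; Each tick turns the controller's Y offset from the grab point into a clamped Scene yaw and passes the clamped angle to BPBreech's Load.
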(event OnGrabbed(GrabComponent)
  (params (MotionControllerRight :type Motion%20Controller%20Component%20Object%20Reference) (MotionControllerLeft :type Motion%20Controller%20Component%20Object%20Reference))
  (Variables|Default|SetMotion%20Controller 0)
  (Utilities|Time|SetTimerbyFunctionName 0 "EventBeginStep" 0.02 true)
  (Rendering|SetVisibility (Variables|Default|GetHand) true false))

(event OnDropped(GrabComponent)
  (Variables|Default|SetMotion%20Controller 0)
  (Utilities|Time|ClearTimerbyFunctionName 0 "EventBeginStep")
  (Rendering|SetVisibility (Variables|Default|GetHand) false false))

(event EventBeginPlay
  (|CallParentFunction)
  (Rendering|SetVisibility (Variables|Default|GetHand) false false))

(fn ConstructionScript
  (|CallParentFunction))

(fn EventBeginStep
  (bind _scene (Variables|Default|GetScene))
  (bind _motion_controller (Variables|Default|GetMotion%20Controller))
  (bind _grabcomponent (Variables|Default|GetGrabComponent))
  (bind _returnvalue (Transformation|GetWorldTransform _motion_controller))
  (bind _returnvalue_2 (Transformation|GetWorldTransform _grabcomponent))
  (bind _relativerotation (Variables|/Script/Engine.SceneComponent|GetRelativeRotation _scene))
  (bind _relativelocation (Variables|/Script/Engine.SceneComponent|GetRelativeLocation _grabcomponent))
  (bind _returnvalue_3 (Math|Transform|MakeRelativeTransform _returnvalue _returnvalue_2))
  (bind _returnvalue_4 (- _relativelocation (.location _returnvalue_3)))
  (bind _returnvalue_5 (- (.yaw _relativerotation) (.y _returnvalue_4)))
  (bind _returnvalue_6 (Math|Float|Clamp(Float) _returnvalue_5 0.0 4e+01))
  (|CallParentFunction)
  (Transformation|SetRelativeRotation _scene (Math|Rotator|MakeRotator (.roll _relativerotation) (.pitch _relativerotation) _returnvalue_6) false false)
  (Default|Load (Variables|Default|GetBP_Breech) _returnvalue_6))

(fn EventEndStep
  (|CallParentFunction))