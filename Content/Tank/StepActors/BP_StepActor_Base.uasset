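; Base actor for step-driven content in the Tank folder, tying each instance to one content state through CurStep.
; On BeginPlay it binds to the GameState's content-state dispatcher.
; UpdateContentStep calls EventBeginStep when the state matches CurStep and ResetStep otherwise, both empty hooks for children.
; EventEndStep asks the GameState to change to EndStep, but only when CurStep equals one specific enum value.
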(event EventBeginPlay
  (CallFunction|BindGameState))

(fn ConstructionScript)

(fn BindGameState
  (bind _asbp_game_state (Utilities|Casting|CastToBP_GameState (Game|GetGameState)))
  (EventDispatchers|BindEventtoEventDispatcherContentState _asbp_game_state (EventDispatchers|CreateEvent :!event UpdateContentStep)))

(fn UpdateContentStep
  (params (ContentState :type EN_FireSequence%20Enum :default "NewEnumerator0"))
  (if (Utilities|Enum|Equal(Enum) ContentState (Variables|Default|GetCurStep))
    (CallFunction|EventBeginStep)
    (else
      (CallFunction|ResetStep))))

(fn EventBeginStep)

(fn EventEndStep
  (if (Utilities|Enum|Equal(Enum) (Variables|Default|GetCurStep) "NewEnumerator3")
    (bind _asbp_game_state (Utilities|Casting|CastToBP_GameState (Game|GetGameState)))
    (Default|ChangeContentState _asbp_game_state (Variables|Default|GetEndStep))))

(fn ResetStep)